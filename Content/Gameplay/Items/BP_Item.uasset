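; BP_Item is a data-driven pickup actor whose mesh, material, transform, light color and optional rotation come from an Items data table row.
; The construction script calls Init with the ItemID, which looks up the row and applies it, printing a message if none is found.
; On mesh overlap, it offers itself to actors implementing IRunCharacter; if accepted, it plays a type-based pickup sound and destroys itself.
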(event `self.StaticMesh.OnComponentBeginOverlap`
  (params (OverlappedComponent :type "PrimitiveComponent Object Reference") (OtherActor :type "Actor Object Reference") (OtherComp :type "PrimitiveComponent Object Reference") (OtherBodyIndex :type Integer) (bFromSweep :type Boolean) (SweepResult :type "HitResult Structure (by ref)"))
  (bind (_name _lightcolor _mesh _material _meshtransform _rotate _statchange _itemchange _pickupsoundtype) (break `/Game/Gameplay/Items/ItemDefinition` (`self.ItemDefinition`)))
  (if (`KismetSystemLibrary.DoesImplementInterface` OtherActor "/Game/Player/IRunCharacter.IRunCharacter_C")
    (bind _pickedup (message `/Game/Gameplay/Items/IItemPicker.PickupItem` OtherActor self))
    (if _pickedup
      (`GameplayStatics.PlaySoundAtLocation` (select `/Game/Gameplay/Items/PickupSoundType` _pickupsoundtype :`NewEnumerator0` "/Game/Audio/270405__littlerobotsoundfactory__pickup-gold-03-new.270405__littlerobotsoundfactory__pickup-gold-03-new" :`NewEnumerator1` "/Game/Audio/126418__cabeeno-rossley__button-select.126418__cabeeno-rossley__button-select" :!type "SoundBase Object Reference") (`self.K2_GetActorLocation`) (struct) (select `/Game/Gameplay/Items/PickupSoundType` _pickupsoundtype :`NewEnumerator0` 0.7 :`NewEnumerator1` 1.3 :!type "Float (single-precision)") 1.0 0.0 null "/Game/Audio/PIckupConcurrency.PIckupConcurrency" OtherActor)
      (`self.K2_DestroyActor`))))

(event `self.Init`
  (params (ItemID :type Name))
  (bind _staticmesh (`self.StaticMesh`))
  (bind _output_get (set `self.ItemID` ItemID))
  (bind _returnvalue (`|GetDataTableRow` "/Game/Gameplay/Items/Items.Items" _output_get)
    (:`then`
      (set `self.ItemDefinition` _returnvalue)
      (bind (_name _lightcolor _mesh _material _meshtransform _rotate) (break `/Game/Gameplay/Items/ItemDefinition` _returnvalue))
      (set `self.Name` _name)
      (if _rotate
        (`AddComponent|NODE_AddRotatingMovementComponent-0`))
      (`LightComponent.SetLightColor` (`self.SpotLight`) _lightcolor true)
      (`StaticMeshComponent.SetStaticMesh` _staticmesh _mesh)
      (`PrimitiveComponent.SetMaterial` _staticmesh 0 _material)
      (`SceneComponent.K2_SetRelativeTransform` _staticmesh _meshtransform false true))
    (:`RowNotFound`
      (`KismetSystemLibrary.PrintString` (`KismetStringLibrary.Concat_StrStr` "ItemID not found: " (`KismetStringLibrary.Conv_NameToString` (`self.ItemID`)))))))

(fn `UserConstructionScript`
  (bind _itemid (`self.ItemID`))
  (if (!= _itemid "None")
    (`self.Init` _itemid)))