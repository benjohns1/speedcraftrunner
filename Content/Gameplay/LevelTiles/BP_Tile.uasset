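; Level tile for a runner game that randomly populates itself with obstacles and items and exposes an attach transform.
; Construction rolls for one obstacle at a child attach point and scatters weighted item picks inside a box, all as child actors.
; The first runner overlap notifies the character, optionally storing its current respawn point.
; Save and Load record and rebuild the child actors and overlap flags, handling only base obstacle and item classes.
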(event `self.TileBounds.OnComponentBeginOverlap`
  (params (OverlappedComponent :type "PrimitiveComponent Object Reference") (OtherActor :type "Actor Object Reference") (OtherComp :type "PrimitiveComponent Object Reference") (OtherBodyIndex :type Integer) (bFromSweep :type Boolean) (SweepResult :type "HitResult Structure (by ref)"))
  (if (`self.OverlapTriggered`)
    _
    (elif (`KismetSystemLibrary.DoesImplementInterface` OtherActor "/Game/Player/IRunCharacter.IRunCharacter_C")
      (set `self.OverlapTriggered` true)
      (if (`self.SaveRespawnTransform`)
        (bind _respawnpoint (message `/Game/Player/IRunCharacter.GetCurrentRespawnPoint` OtherActor))
        (set `self.RespawnPoint` _respawnpoint))
      (message `/Game/Player/IRunCharacter.TileEntered` OtherActor self))))

(fn `GetAttachTransform`
  (returns (AttachTransform :type "Transform Structure") (Done :type Boolean))
  (return (`self.AttachTransform`) false))

(fn `Load`
  (params (SaveGame :type "/Game/Gameplay/Savegame/RunSaveGame Object Reference (by ref)") (PrevObjName :type String))
  (returns (Success :type Boolean))
  (bind (_class _transform _bp_obstacles _bp_items _overlaptriggered _saverespawntransform) (break `/Game/Gameplay/Savegame/SaveStructs/Save_BP_Tile` (`BlueprintMapLibrary.Map_Find` (`/Game/Gameplay/Savegame/RunSaveGame.BP_Tile` SaveGame) PrevObjName)))
  (set `self.OverlapTriggered` _overlaptriggered)
  (set `self.SaveRespawnTransform` _saverespawntransform)
  (bind (_key _value) (`/Game/Utility/ObjectMacros.ForEachStringMap` _bp_obstacles)
    (:`LoopBody`
      (bind (_class_2 _transform_2) (break `/Game/Gameplay/Savegame/SaveStructs/Save_BP_Obstacle` _value))
      (if (== _class_2 "/Game/Gameplay/Obstacles/BP_Obstacle.BP_Obstacle_C")
        (`self.AddObstacle` _transform_2)
        (else
          (`KismetSystemLibrary.PrintString` "ERROR: Obstacle subclasses not handled!"))))
    (:`Completed`
      (bind (_key_2 _value_2) (`/Game/Utility/ObjectMacros.ForEachStringMap` _bp_items)
        (:`LoopBody`
          (bind (_class_3 _transform_3 _itemid) (break `/Game/Gameplay/Savegame/SaveStructs/Save_BP_Item` _value_2))
          (if (== _class_3 "/Game/Gameplay/Items/BP_Item.BP_Item_C")
            (`self.AddItem` _itemid _transform_3)
            (else
              (`KismetSystemLibrary.PrintString` "ERROR: Item subclasses not handled!"))))
        (:`Completed`
          (return true))))))

(fn `Save`
  (params (SaveGame :type "/Game/Gameplay/Savegame/RunSaveGame Object Reference (by ref)"))
  (returns (Success :type Boolean))
  (locals (Obstacles :type "Map of String to /Game/Gameplay/Savegame/SaveStructs/Save_BP_Obstacle Structure") (Items :type "Map of String to /Game/Gameplay/Savegame/SaveStructs/Save_BP_Item Structure"))
  (for _array_element (`self.GetAllChildActors` true)
    (`/Engine/EditorBlueprintResources/StandardMacros.IsValid` _array_element
      (:`Is Valid`
        (bind _returnvalue (`self.GetParentComponent` _array_element))
        (`/Engine/EditorBlueprintResources/StandardMacros.IsValid` _returnvalue
          (:`Is Valid`
            (bind _asbp_obstacle (cast `/Game/Gameplay/Obstacles/BP_Obstacle` _array_element)
              (:`then`
                (bind _returnvalue_2 (`KismetSystemLibrary.GetObjectName` _array_element))
                (bind _returnvalue_3 (`SceneComponent.GetRelativeTransform` _returnvalue))
                (`BlueprintMapLibrary.Map_Add` (`local.Obstacles`) _returnvalue_2 (make `/Game/Gameplay/Savegame/SaveStructs/Save_BP_Obstacle` (`GameplayStatics.GetObjectClass` _asbp_obstacle) _returnvalue_3)))
              (:`CastFailed`
                (bind _asbp_item (cast `/Game/Gameplay/Items/BP_Item` _array_element))
                (`BlueprintMapLibrary.Map_Add` (`local.Items`) _returnvalue_2 (make `/Game/Gameplay/Savegame/SaveStructs/Save_BP_Item` (`GameplayStatics.GetObjectClass` _asbp_item) _returnvalue_3 (`/Game/Gameplay/Items/BP_Item.ItemID` _asbp_item))))))))))
  (`BlueprintMapLibrary.Map_Add` (`/Game/Gameplay/Savegame/RunSaveGame.BP_Tile` SaveGame) (`KismetSystemLibrary.GetObjectName` self) (make `/Game/Gameplay/Savegame/SaveStructs/Save_BP_Tile` (`GameplayStatics.GetObjectClass` self) (`self.GetTransform` self) (`local.Obstacles`) (`local.Items`) (`self.OverlapTriggered`) (`self.SaveRespawnTransform`)))
  (return true))

(fn `SpawnItem`
  (params (ItemID :type Name))
  (locals (SpawnLocation :type "Vector Structure"))
  (bind _itemarea (`self.ItemArea`))
  (`self.AddItem` ItemID (`KismetMathLibrary.MakeTransform` (`KismetMathLibrary.RandomPointInBoundingBox` (`SceneComponent.RelativeLocation` _itemarea) (`BoxComponent.BoxExtent` _itemarea)))))

(fn `SpawnItems`
  (for _array_element (`self.ItemSpawnConfigs`)
    (bind (_amountmin _amountmax _itemoptions _spawnchance) (break `/Game/Gameplay/Items/ItemSpawnProbabilityCache` _array_element))
    (if (`KismetMathLibrary.RandomBoolWithWeight` _spawnchance)
      (for _ (range (`KismetMathLibrary.RandomIntegerInRange` _amountmin _amountmax))
        (`self.SpawnItem` (`/Game/Utility/ObjectMacros.GetRandomItemInArray` _itemoptions))))))

(fn `SpawnObstacle`
  (bind _obstacletransforms (`self.ObstacleTransforms`))
  (if (`KismetMathLibrary.RandomBoolWithWeight` (`self.ObstacleChance`))
    (`self.AddObstacle` (`|GetArrayItem` _obstacletransforms (`KismetMathLibrary.RandomIntegerInRange` 0 (`KismetArrayLibrary.Array_LastIndex` _obstacletransforms))))))

(fn `UserConstructionScript`
  ;[1 1 1] Obstacle attach points
  (for _array_element (`SceneComponent.GetChildrenComponents` (`self.ObstacleAttachments`) false)
    (`KismetArrayLibrary.Array_Add` (`self.ObstacleTransforms`) (`SceneComponent.GetRelativeTransform` _array_element)))
  ;[1 1 1] Spawn items and obstacles
  (`self.SpawnObstacle`)
  (`self.SpawnItems`)
  ;[1 1 1] Tile attach points
  (set `self.AttachTransform` (`SceneComponent.K2_GetComponentToWorld` (`self.AttachPoint`))))