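; Small checkpoint level tile Blueprint that shows a save gate only when the tile saves a respawn transform.
; The construction script runs the parent's logic, then checks SaveRespawnTransform.
; When that flag is off, it collects the Gate component's direct children into ComponentsToDestroy and destroys them in a second loop, leaving Gate itself in place.
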(fn `UserConstructionScript`
  (locals (ComponentsToDestroy :type "Array of SceneComponent Object Reference"))
  (`parent.UserConstructionScript`)
  ;[1 1 1] Remove save gate if no save should occur on this tile
  (if (not (`self.SaveRespawnTransform`))
    (for _array_element (`SceneComponent.GetChildrenComponents` (`self.Gate`) false)
      (`KismetArrayLibrary.Array_Add` (`local.ComponentsToDestroy`) _array_element))
    (for _array_element_2 (`local.ComponentsToDestroy`)
      (`ActorComponent.K2_DestroyComponent` _array_element_2))))