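; Themed sky sphere that recolors its sky material to match a given Theme.
; SetTheme stores the theme and pushes its primary color to the horizon and overall color parameters, and its secondary color to the zenith.
; The construction script only calls the parent's, and GetTheme has no logic.
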(event `/Game/Environment/ITheme.SetTheme`
  (params (Theme :type "/Game/Environment/Theme Structure"))
  (bind _output_get (set `self.Theme` Theme))
  (bind (_primarycolor _secondarycolor) (break `/Game/Environment/Theme` _output_get))
  (`MaterialInstanceDynamic.SetVectorParameterValue` (`self.Sky material`) "Horizon color" _primarycolor)
  (`MaterialInstanceDynamic.SetVectorParameterValue` (`self.Sky material`) "Overall color" _primarycolor)
  (`MaterialInstanceDynamic.SetVectorParameterValue` (`self.Sky material`) "Zenith color" _secondarycolor))

(fn `GetTheme`
  (returns (Theme :type "/Game/Environment/Theme Structure"))
  (return))

(fn `UserConstructionScript`
  (`parent.UserConstructionScript`))