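; BP_ThemedFogLighting is an environment Blueprint that recolors fog and lighting from a color theme.
; SetTheme stores the theme, then applies its primary color to fog inscattering and the sky light, and its secondary color to directional inscattering and the sun light.
; The accent color becomes the sun's bloom tint, and GetTheme returns the stored theme.
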(event `/Game/Environment/ITheme.SetTheme`
  (params (Theme :type "/Game/Environment/Theme Structure"))
  (bind _output_get (set `self.Theme` Theme))
  (bind (_primarycolor _secondarycolor _accentcolor) (break `/Game/Environment/Theme` _output_get))
  (`ExponentialHeightFogComponent.SetFogInscatteringColor` (`self.Fog`) _primarycolor)
  (`SkyLightComponent.SetLightColor` (`self.SkyLight`) _primarycolor)
  (`ExponentialHeightFogComponent.SetDirectionalInscatteringColor` (`self.Fog`) _secondarycolor)
  (`LightComponent.SetLightColor` (`self.SunLight`) _secondarycolor true)
  (`LightComponent.SetBloomTint` (`self.SunLight`) (`KismetMathLibrary.Conv_LinearColorToColor` _accentcolor)))

(fn `GetTheme`
  (returns (Theme :type "/Game/Environment/Theme Structure"))
  (return (`self.Theme`)))

(fn `UserConstructionScript`)